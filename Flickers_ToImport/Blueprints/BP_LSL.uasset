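; BP_LSL bridges the flicker-based game and Timeflux over Lab Streaming Layer.
; On BeginPlay it announces the session and binds to the flicker manager, calibration and cup-task Blueprints' dispatchers.
; Outlets push epoch markers (bit during calibration, index otherwise) and changed codes.
; Inlets rebroadcast first-received code sequences, the model-ready signal and target predictions, extracted from raw strings by digit filtering, as events.
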(event OnStreamUpdatedString(LSLInlet_Sequence)
  (params (StringArray :type Array%20of%20Strings) (DeltaSeconds :type Float%20%28single-precision%29))
  (if (not (Variables|Default|GetSequenceAlreadyStreamed))
    (Variables|Default|SetSequenceAlreadyStreamed true)
    (Utilities|FlowControl|Sequence
      (:then_0
        (Default|CallCalibrationSequencesReceived (Utilities|Array|Get(acopy) StringArray)))
      (:then_1
        (Default|CallTaskSequencesReceived (Utilities|Array|Get(acopy) StringArray 1))))))

(event OnStreamUpdatedString(LSLInlet_Events)
  (params (StringArray :type Array%20of%20Strings) (DeltaSeconds :type Float%20%28single-precision%29))
  (for _array_element StringArray
    (if (Utilities|Enum|Equal(Enum) _array_element "ready")
      (Default|CallReadyEventReceived))))

(event OnStreamUpdatedString(LSLInlet_Predictions)
  (params (StringArray :type Array%20of%20Strings) (DeltaSeconds :type Float%20%28single-precision%29))
  (bind _output (Utilities|Array|Get(acopy) StringArray 1))
  (bind _returnvalue (Utilities|String|FindSubstring _output "\"target\"" false false 0))
  (bind _returnvalue_2 (- _returnvalue 7))
  (bind _returnvalue_3 (Utilities|String|Right _output _returnvalue_2))
  (bind _returnvalue_4 (Utilities|String|FindSubstring _returnvalue_3 "frames" false false 0))
  (bind _returnvalue_5 (Utilities|String|LeftChop _returnvalue_3 _returnvalue_4))
  ;[1 1 1] Since Timeflux sends the Predictions with this format: ...  "target": self._current_target,  "frames": str(self._frames), ..., we clear it to just obtain the value of the target
  (Variables|Default|SetTargetPrediction "")
  (for _index (range 0 (Utilities|String|Len _returnvalue_5))
    (if (Class|KismetStringLibrary|IsNumeric (Utilities|String|GetSubstring _returnvalue_5 _index))
      (Variables|Default|SetTargetPrediction (Utilities|String|Append (Variables|Default|GetTargetPrediction) (Utilities|String|GetSubstring _returnvalue_5 _index)))))
  (Default|CallPredictionReceived (Variables|Default|GetTargetPrediction)))

(event Custom|Send%20Codes%20that%20changed%20their%20object
  (params (NewParam :type String))
  (Utilities|Array|SetArrayElem (Variables|Default|GetOutletData_codesChanged) 1 NewParam true)
  (Class|LSLOutletComponent|PushSampleString (Variables|Default|GetLSLOutlet_CodesChanged) (Variables|Default|GetOutletData_codesChanged)))

(event Custom|CustomEvent_9
  ;[1 1 1] Bind with other bluprints events. When this events are triggered in their respective blueprints, the BP_LSL triggers its own events
  (Variables|Default|SetCalibrationPhase false)
  (CallFunction|SendDataEpochs))

(event Custom|Send_DataEpochs
  (Class|LSLOutletComponent|PushSampleString (Variables|Default|GetLSLOutlet_Epochs) (Variables|Default|GetOutletData_epochs)))

(event Custom|EpochAnalysis
  (params (bit :type Integer) (index :type Integer))
  (bind _outletdata_epochs (Variables|Default|GetOutletData_epochs))
  (Utilities|Array|SetArrayElem (Variables|Default|GetOutletData_epochs) 0 "epoch")
  (if (Variables|Default|GetCalibrationPhase)
    (Utilities|Array|SetArrayElem _outletdata_epochs 1 (Utilities|String|Append "bit:" (Utilities|String|ToString(Integer) bit)))
    (else
      (Utilities|Array|SetArrayElem _outletdata_epochs 1 (Utilities|String|Append "index:" (Utilities|String|ToString(Integer) index)))))
  (CallFunction|SendDataEpochs))

(event Custom|CustomEvent_8
  ;[1 1 1] Bind with other bluprints events. When this events are triggered in their respective blueprints, the BP_LSL triggers its own events
  (Variables|Default|SetCalibrationPhase true)
  (CallFunction|SendDataEpochs))

(event EventBeginPlay
  (Utilities|FlowControl|Sequence
    (:then_0
      (Utilities|Array|SetArrayElem (Variables|Default|GetOutletData_epochs) 0 "session_begins" true)
      (CallFunction|SendDataEpochs))
    (:then_1
      ;[1 1 1] Bind with other bluprints events. When this events are triggered in their respective blueprints, the BP_LSL triggers its own events
      (bind _returnvalue (Actor|GetActorOfClass "/Game/Flickers_ToImport/Blueprints/BP_FlickerManager.BP_FlickerManager_C"))
      (Utilities|FlowControl|Sequence
        (:then_0
          (EventDispatchers|BindEventtoEpoch _returnvalue (EventDispatchers|CreateEvent :!event Custom|EpochAnalysis)))
        (:then_1
          (EventDispatchers|BindEventtoCodesChanged _returnvalue (EventDispatchers|CreateEvent :!event Custom|Send%20Codes%20that%20changed%20their%20object)))))
    (:then_2
      (bind _returnvalue_2 (Actor|GetActorOfClass "/Game/Flickers_ToImport/Blueprints/BP_CalibrationDYNAMIC.BP_CalibrationDYNAMIC_C"))
      (Utilities|FlowControl|Sequence
        (:then_0
          (EventDispatchers|BindEventtoCalibrationBegins _returnvalue_2 (delegate Custom|CustomEvent_8)))
        (:then_1
          (EventDispatchers|BindEventtoCalibrationEnds _returnvalue_2 (delegate Custom|CustomEvent_9)))))
    (:then_3
      ;[1 1 1] IMPORTANT: If any blueprint wants to send information thorugh LSL to Timeflux, and therefore communicate to this blueprint through event dispatchers, those bluerpints have to be called in here, and connected to the events that they should trigger within the BP_LSL
      (bind _returnvalue_3 (Actor|GetActorOfClass "/Game/Flickers_ToImport/Blueprints/BP_ChooseWhateverCupDYNAMIC.BP_ChooseWhateverCupDYNAMIC_C"))
      (Utilities|FlowControl|Sequence
        (:then_0
          (EventDispatchers|BindEventtoTaskBegins _returnvalue_3 (EventDispatchers|CreateEvent :!event Custom|Send_DataEpochs)))
        (:then_1
          (EventDispatchers|BindEventtoReset _returnvalue_3 (EventDispatchers|CreateEvent :!event Custom|Send_DataEpochs)))
        (:then_2
          (EventDispatchers|BindEventtoTaskEnds _returnvalue_3 (EventDispatchers|CreateEvent :!event Custom|Send_DataEpochs)))))
    (:then_4
      (bind _returnvalue_4 (Actor|GetActorOfClass "/Game/Flickers_ToImport/Blueprints/BP_CupsDynamic.BP_CupsDynamic_C"))
      (Utilities|FlowControl|Sequence
        (:then_0
          (EventDispatchers|BindEventtoTaskBegins _returnvalue_4 (EventDispatchers|CreateEvent :!event Custom|Send_DataEpochs)))
        (:then_1
          (EventDispatchers|BindEventtoReset _returnvalue_4 (EventDispatchers|CreateEvent :!event Custom|Send_DataEpochs)))
        (:then_2
          (EventDispatchers|BindEventtoTaskEnds _returnvalue_4 (EventDispatchers|CreateEvent :!event Custom|Send_DataEpochs)))))))

(fn ConstructionScript)