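; Blueprint for a flicker-based cup selection task in a shell game, driven by Timeflux through BP_LSL.
; BeginPlay binds BP_LSL's task-sequence, ready and prediction events.
; ChooseCup signals run start, reveals components and has BP_FlickerManager flicker "Flicker"-tagged objects using received sequences.
; Each prediction pauses flickering, highlights meshes of the matching code sequence, then resumes without rebuilding sequences and restores their dynamic material.
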(event Custom|ChooseCup
  ;[1 1 1] Timeflux gets notify
  (Utilities|Array|SetArrayElem (Variables|/Game/Flickers_ToImport/Blueprints/BP_LSL.BP_LSL_C|GetOutletData_epochs (Variables|Components|GetBP_LSL)) 0 "run_begins")
  (Default|CallTaskBegins)
  (Utilities|FlowControl|Delay 0.5)
  (Utilities|FlowControl|Sequence
    (:then_0
      (Development|PrintString "Start_ShellGame")
      (Rendering|SetVisibility (Variables|Default|GetDefaultSceneRoot) true true)
      (Rendering|SetVisibility (Variables|Default|GetRotationPt) false true))
    (:then_1
      (Default|FlickerEverythingwithThisTag (Variables|Components|GetFlickerManager) "Flicker" (Variables|Default|GetTaskSeqsRec) true))))

(event Custom|PredictionRecieved
  (params (target :type String))
  ;[1 1 1] Once we get a prediction, the flickering stops
  (Utilities|FlowControl|Sequence
    (:then_0
      (Default|StopFlickering (Variables|Components|GetFlickerManager) true false) ; Stop without the reset of the sequences, so the set up flickers doesn't have to be done again
    )
    (:then_1
      (Development|PrintString (Utilities|String|Append "PREDICTION TARJET:" target))
      (Variables|Default|SetPrediction "")
      (Variables|Default|SetPredictionMatches false)
      (bind _array_element (Utilities|Array|ForEachLoopwithBreak (Variables|/Game/Flickers_ToImport/Blueprints/BP_FlickerManager.BP_FlickerManager_C|GetStruct_FlickerCodeSequences (Variables|Components|GetFlickerManager)))
        (:LoopBody
          ;[1 1 1] Checks what code sequence correspond to the prediction target
          (if (== (.SequenceID (Utilities|Struct|BreakStruct_FlickerSequence _array_element)) target)
            (Variables|Default|SetPrediction _array_element)
            (Variables|Default|SetPredictionMatches true)))
        (:Completed
          ;[1 1 1] Sets a new overlay material to the mesh components linked to that code sequence, so the user can see whatwas being selected
          (if (Variables|Default|GetPredictionMatches)
            (Development|PrintString (Utilities|String|ToString(Integer) (.SequenceID (Utilities|Struct|BreakStruct_FlickerSequence (Variables|Default|GetPrediction)))))
            (for _array_element_2 (.AssociatedMeshComponents (Utilities|Struct|BreakStruct_FlickerSequence (Variables|Default|GetPrediction)))
              (Development|PrintString (Utilities|GetDisplayName _array_element_2))
              (Rendering|Material|SetOverlayMaterial _array_element_2 "/Game/FPWeapon/Materials/FirstPersonProjectileMaterial.FirstPersonProjectileMaterial" :!class /Script/Engine.MeshComponent))
            (else
              (Development|PrintString "THE PREDICTION DOESNT MATCH!!!!")))
          ;[1 1 1] After a delay, flickering start again, and therefore the overlay signaling material is removed
          (Utilities|FlowControl|Delay (Variables|Default|GetPredictionPause))
          (Default|FlickerEverythingwithThisTag (Variables|Components|GetFlickerManager) "Flicker" "" false)
          (for _array_element_3 (.AssociatedMeshComponents (Utilities|Struct|BreakStruct_FlickerSequence (Variables|Default|GetPrediction)))
            (Rendering|Material|SetOverlayMaterial _array_element_3 (.DynamicMaterial (Utilities|Struct|BreakStruct_FlickerSequence (Variables|Default|GetPrediction))) :!class /Script/Engine.MeshComponent)))))))

(event Custom|CustomEvent
  (params (TaskSeqsRec :type String))
  ;[1 1 1] Retrieves BP_LSL and BP_FlickerManager actors. Once both the Tasks seqs and the Ready Event are received the game starts
  (Variables|Default|SetTaskSeqsRec TaskSeqsRec))

(event EventBeginPlay
  (Utilities|FlowControl|Sequence
    (:then_0
      (Rendering|SetVisibility (Variables|Default|GetDefaultSceneRoot) false true)
      (Rendering|SetVisibility (Variables|Default|GetM_Cup) true true))
    (:then_1
      ;[1 1 1] Retrieves BP_LSL and BP_FlickerManager actors. Once both the Tasks seqs and the Ready Event are received the game starts
      (bind _returnvalue (Actor|GetActorOfClass "/Game/Flickers_ToImport/Blueprints/BP_FlickerManager.BP_FlickerManager_C"))
      (Variables|Components|SetFlickerManager _returnvalue))
    (:then_2
      (bind _returnvalue_2 (Actor|GetActorOfClass "/Game/Flickers_ToImport/Blueprints/BP_LSL.BP_LSL_C"))
      (Variables|Components|SetBP_LSL _returnvalue_2)
      (Utilities|FlowControl|Sequence
        (:then_0
          (EventDispatchers|BindEventtoTaskSequencesReceived (Variables|Components|GetBP_LSL) (delegate Custom|CustomEvent)))
        (:then_1
          (EventDispatchers|BindEventtoReadyEventReceived (Variables|Components|GetBP_LSL) (EventDispatchers|CreateEvent :!event Custom|ChooseCup)) ; The game wont start until Timeflux sends "ready" event
        )
        (:then_2
          (EventDispatchers|BindEventtoPredictionReceived (Variables|Components|GetBP_LSL) (EventDispatchers|CreateEvent :!event Custom|PredictionRecieved)))))))

(fn ConstructionScript)