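; BP_FlickerManager flickers tagged mesh components with Timeflux bit sequences, for calibration and gameplay.
; Setup groups components by paired actor/component tags and gives each parsed sequence its own dynamic material.
; A perception timer filters groups by FOV and subdivided line-of-sight traces, then assigns the nearest to sequences as overlay materials, reporting changes via CodesChanged.
; A flicker timer sets each material's Visibility from the current bit and calls Epoch with bit and index.
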(event Custom|SetUp_Flickers
  (params (Tag :type Name :default "Flicker") (Timeflux_sequenceString :type String) (Patches_Visible :type Boolean))
  (bind _mapperceptiondata (CallFunction|GetMeshComponentsbyTag Tag))
  (Variables|Default|SetMapPerceptionData _mapperceptiondata)
  (bind (_itotalsequences _arrsequenceswithoutmaterial) (CallFunction|ParseStringtoFlickerSequenceStructs Timeflux_sequenceString))
  (Variables|Default|SetTotalCodeSequences _itotalsequences)
  (bind _arrsequenceswithmaterialmapping (CallFunction|AssignDynamicMaterialtoFlickerSequence _arrsequenceswithoutmaterial Patches_Visible))
  (Variables|Default|SetStruct_FlickerCodeSequences _arrsequenceswithmaterialmapping)
  (bind _arrmindistances (CallFunction|SetPerceptionData (Variables|Default|GetMapPerceptionData)))
  (CallFunction|ArrangeIntoCodesStruct (Variables|Default|GetMapPerceptionData) _arrmindistances (Variables|Default|GetStruct_FlickerCodeSequences)))

(event Custom|ResetCodeSequences
  (Utilities|Array|Clear (Variables|Default|GetStruct_FlickerCodeSequences)))

(event Custom|Pause_Flickering
  (params (TimePaused :type Float%20%28double-precision%29) (Reset%20IndexCode :type Boolean))
  (Utilities|FlowControl|Sequence
    (:then_0
      (CallFunction|StopFlickering Reset%20IndexCode false))
    (:then_1
      (Utilities|FlowControl|Delay TimePaused)
      (CallFunction|FlickerEverythingwithThisTag "Flicker" "0" false) ; It doesn't matter the tag and the sequence (used in the setup), because here is just a pause, s the setup wont be done again
    )))

(event Custom|DynamicChosingComponents
  (bind _mapperceptiondata (Variables|Default|GetMapPerceptionData))
  (bind _arrmindistances (CallFunction|SetPerceptionData _mapperceptiondata))
  (bind _scodesthatchangecomponents (CallFunction|ArrangeIntoCodesStruct _mapperceptiondata _arrmindistances (Variables|Default|GetStruct_FlickerCodeSequences)))
  (if (not (Utilities|Array|IsEmpty _scodesthatchangecomponents))
    (Default|CallCodesChanged _scodesthatchangecomponents)))

(event Custom|Stop_Flickering
  (params (Reset%20IndexCode :type Boolean) (Reset%20CodeSequences :type Boolean))
  (Utilities|Time|ClearTimerbyFunctionName 0 "DynamicChosingComponents")
  (Utilities|Time|ClearTimerbyFunctionName 0 "E_UpdateBlink")
  (for _array_element (Variables|Default|GetStruct_FlickerCodeSequences)
    (Rendering|Material|SetScalarParameterValue (Utilities|Struct|BreakStruct_FlickerSequence _array_element) "Visibility" 0.0 :!class /Script/Engine.MaterialInstanceDynamic))
  (Utilities|FlowControl|Sequence
    (:then_0
      (if Reset%20IndexCode
        (Variables|Default|SetBitIndex 0)))
    (:then_1
      (if Reset%20CodeSequences
        (CallFunction|ResetCodeSequences)))))

(event Custom|E_UpdateBlink
  (Utilities|FlowControl|Sequence
    (:then_0
      (bind (_ibit _ilastupdatedbitinde) (CallFunction|UpdateFlickerSequences (Variables|Default|GetStruct_FlickerCodeSequences))))
    (:then_1
      (Default|CallEpoch _ibit _ilastupdatedbitinde))))

(event Custom|Flicker_everything_with_this_Tag
  (params (Tag :type Name :default "Flicker") (Timeflux_sequenceString :type String) (SetUpFlickers :type Boolean))
  (bind _flickerrate (Variables|Default|GetFlickerRate))
  (bind _perceptionupdaterate (Variables|Default|GetPerceptionUpdateRate))
  (if SetUpFlickers
    (CallFunction|SetUpFlickers Tag Timeflux_sequenceString false))
  (Utilities|Time|SetTimerbyEvent (EventDispatchers|CreateEvent :!event Custom|DynamicChosingComponents) _perceptionupdaterate true (- 0.0 _perceptionupdaterate))
  (Utilities|Time|SetTimerbyEvent (EventDispatchers|CreateEvent :!event Custom|E_UpdateBlink) _flickerrate true (- 0.0 _flickerrate)))

(fn ConstructionScript)

(fn StringSequencetoArrayIntSequence
  (params (sInputString :type String))
  (for _index (range 0 (- (Utilities|String|Len sInputString) 1))
    (if (Class|KismetStringLibrary|IsNumeric (Utilities|String|GetSubstring sInputString _index))
      (Utilities|Array|Add (LocalVariables|GetArrNumericValue%20) (Math|Conversions|ToInteger(Byte) (Utilities|String|GetSubstring sInputString _index)))))
  (Variables|Default|SetSingleSequenceLength (Utilities|Array|Length (LocalVariables|GetArrNumericValue%20)))
  (return (LocalVariables|GetArrNumericValue%20)))

(fn ParseStringtoFlickerSequenceStructs
  (params (sTimefluxSequence%20 :type String))
  (bind _delimitertimefluxsequences (Variables|Default|GetDelimiterTimefluxSequences))
  (bind _returnvalue (Utilities|String|ParseIntoArray sTimefluxSequence%20 _delimitertimefluxsequences false))
  (for (_array_element _array_index) _returnvalue
    (bind _arrnumericvalues (CallFunction|StringSequencetoArrayIntSequence _array_element))
    (Utilities|Array|Add (LocalVariables|GetArrFlickerSequences) (Utilities|Struct|MakeStruct_FlickerSequence _array_index _arrnumericvalues)))
  (return (Utilities|Array|Length _returnvalue) (LocalVariables|GetArrFlickerSequences)))

(fn AssignDynamicMaterialtoFlickerSequence
  (params (ArrSequencesWithoutMaterial :type Array%20of%20Struct%20Flicker%20Sequence%20Structures) (bPatchesVisible :type Boolean))
  (if bPatchesVisible
    (LocalVariables|SetPatchesVisibility 1.0)
    (else
      (LocalVariables|SetPatchesVisibility 0.0)))
  (for _array_element ArrSequencesWithoutMaterial
    (bind _returnvalue (Rendering|Material|CreateDynamicMaterialInstance (Variables|Default|GetDM_FlickerMaterialInstance) (Utilities|String|StringToName (Utilities|String|ToString(Integer) (Utilities|Struct|BreakStruct_FlickerSequence _array_element))) "Transient" :!class /Script/Engine.KismetMaterialLibrary))
    (Rendering|Material|SetScalarParameterValue _returnvalue "Visibility" (LocalVariables|GetPatchesVisibility) :!class /Script/Engine.MaterialInstanceDynamic)
    (bind _structout (Utilities|Struct|SetmembersinStruct_FlickerSequence _array_element _returnvalue))
    (Utilities|Array|SetArrayElem ArrSequencesWithoutMaterial (Utilities|Struct|BreakStruct_FlickerSequence _array_element) _structout true))
  (return ArrSequencesWithoutMaterial))

(fn UpdateFlickerSequences
  (params (ArrFlickerSequencesWithMaterial :type Array%20of%20Struct%20Flicker%20Sequence%20Structures))
  (LocalVariables|SetLastUpdatedBitIndex (Variables|Default|GetBitIndex))
  (for (_array_element _array_index) ArrFlickerSequencesWithMaterial
    ;[1 1 1] During calibration, only one sequence of codes is used, and the system processes a single bit from this sequence to calibrate. During gameplay, only the index is used, and not the bit value
    (if (== _array_index 0)
      (LocalVariables|SetBitFirstCodeSeq (Utilities|Array|Get(acopy) (.Sequence (Utilities|Struct|BreakStruct_FlickerSequence _array_element)) (Variables|Default|GetBitIndex))))
    (Rendering|Material|SetScalarParameterValue (.DynamicMaterial (Utilities|Struct|BreakStruct_FlickerSequence _array_element)) "Visibility" (Math|Conversions|ToFloat(Integer) (Utilities|Array|Get(acopy) (.Sequence (Utilities|Struct|BreakStruct_FlickerSequence _array_element)) (Variables|Default|GetBitIndex))) :!class /Script/Engine.MaterialInstanceDynamic) ; The opacity parameter value  is defined  with the current bit value
  )
  ;[1 1 1] During gameplay, instead of the bit, the system tracks the index (iBitIndex) instead of the bit, as each sequence will have a different bit value
  (bind _result (Math|Integer|IncrementInt (Variables|Default|GetBitIndex))
    (:%20%20
      (if (>= _result (Utilities|Array|Length (.Sequence (Utilities|Struct|BreakStruct_FlickerSequence _array_element))))
        (Variables|Default|SetBitIndex 0) ; The sequence is restarted
      )
      (return (LocalVariables|GetBitFirstCodeSeq) (LocalVariables|GetLastUpdatedBitIndex)))))

(fn GetDistancetoPlayer
  (params (Target :type Scene%20Component%20Object%20Reference))
  (return (Math|Vector|Distance(Vector) (Transformation|GetWorldLocation Target) (Transformation|GetActorLocation (Game|Player|GetPlayerPawn 0)))))

(fn FOVFilter
  (params (TargetMeshComponent :type Mesh%20Component%20Object%20Reference))
  (bind _returnvalue (Game|GetPlayerCameraManager 0))
  (return (>= (Math|Vector|DotProduct (Math|Vector|Normalize (- (Transformation|GetWorldLocation TargetMeshComponent) (Transformation|GetActorLocation _returnvalue)) 1e-05) (Transformation|GetActorForwardVector _returnvalue)) (Math|Trig|Cos(Degrees) (/ (Variables|Default|GetFOV_Angle) 2.0)))))

(fn LineOfSightFilter
  (params (TargetMeshComponent :type Mesh%20Component%20Object%20Reference))
  (bind (_origin _boxextent _sphereradius) (Collision|GetComponentBounds TargetMeshComponent))
  (LocalVariables|SetOrigin _origin)
  (LocalVariables|SetBoxExtent (- _boxextent 5))
  ;[1 1 1] Dynamically determines how many line traces will be used based on the size of the target
  (bind _output_get (LocalVariables|SetNumSubdivisions (Class|LowEntryExtendedStandardLibrary|CeilDecimals (/ _sphereradius (Variables|Default|GetLineOfSightSubdivision)))))
  (LocalVariables|SetTraceSpacing (/ 1.0 _output_get))
  ;[1 1 1] Computes and stores evenly distributed trace directions without scaling them yet
  (for _index (range 0 (- (Math|Float|Ceil (LocalVariables|GetNumSubdivisions)) 1))
    (for _array_element (LocalVariables|GetArrNormalMatrix)
      (Utilities|Array|Add (LocalVariables|GetArrAux) (* _array_element (LocalVariables|GetTraceSpacing) (+ _index 1)))))
  (Utilities|Array|AppendArray (LocalVariables|GetArrNormalMatrix) (LocalVariables|GetArrAux))
  ;[1 1 1] Offsets the scaled vectors using the Origin and stores the final positions in the Key Points array
  (for _array_element_2 (LocalVariables|GetArrNormalMatrix)
    (Utilities|Array|Add (LocalVariables|GetArrKeyPoints) (+ (* _array_element_2 (LocalVariables|GetBoxExtent)) (LocalVariables|GetOrigin))))
  ;[1 1 1] Keeps drawing line traces til any trace confirms visibility. Then the function stops further traces and returns true
  (bind _array_element_3 (Utilities|Array|ForEachLoopwithBreak (LocalVariables|GetArrKeyPoints) :!label _label)
    (:LoopBody
      (bind _outhit (Collision|LineTraceByChannel (Camera|GetCameraLocation (Game|GetPlayerCameraManager 0)) _array_element_3 "TraceTypeQuery1" false (Utilities|Array|MakeArray (Game|Player|GetPlayerPawn 0)) "None"))
      (if (== (.HitComponent (Collision|BreakHitResult _outhit)) TargetMeshComponent)
        (LocalVariables|SetVisible (== (.HitComponent (Collision|BreakHitResult _outhit)) TargetMeshComponent))
        (Utilities|FlowControl|Sequence ; We only draw as many traces as needed to find visibility, but as soon as any detects visible, we don't draw the others
          (:then_0
            (goto _label Break))
          (:then_1
            (return (LocalVariables|GetVisible))))))
    (:Completed
      (return (LocalVariables|GetVisible)))))

(fn GetMeshComponentsbyTag
  (params (Tag%20Studied :type Name))
  (bind _outactors (Actor|GetAllActorswithTag Tag%20Studied))
  (for (_array_element _array_index) _outactors
    ;[1 1 1] Actors can have multiple tags, and their components can also have multiple tags. However, the key rule is that the tag at a specific index in the actor must correspond to the tag at the same index in its components because they are paired together. So we save this index: iTagIndex
    (LocalVariables|SetTagIndex (Utilities|Array|FindItem (Variables|/Script/Engine.Actor|GetTags _array_element) Tag%20Studied))
    (LocalVariables|SetActorIndex _array_index)
    (LocalVariables|SetHasTag false)
    (Utilities|Array|Clear (LocalVariables|GetArrComponentsWithoutTags))
    (for _array_element_2 (Actor|GetComponentsByClass _array_element "/Script/Engine.MeshComponent") ; gets each mesh component of the actor
      (if (== (.Original%20Tag (Utilities|GetandFormatComponentTag _array_element_2 (LocalVariables|GetTagIndex) (LocalVariables|GetActorIndex))) "")
        (Utilities|Array|Add (LocalVariables|GetArrComponentsWithoutTags) _array_element_2)
        (else
          (LocalVariables|SetHasTag true)
          (Utilities|AddComponenttoMapTagComponents (.Format%20Tag%20 (Utilities|GetandFormatComponentTag _array_element_2 (LocalVariables|GetTagIndex) (LocalVariables|GetActorIndex))) _array_element_2 (LocalVariables|GetMapTagComponents)) ; Components are grouped in case they have the same format tag, and saved in the Map Tag Components
        )))
    ;[1 1 1] In case all the components within the actor have "None" for that Actor index, then all the components will flicker using the same code (and they flicker because the actor that contains them was tagged )
    (if (not (LocalVariables|GetHasTag))
      (for _array_element_3 (LocalVariables|GetArrComponentsWithoutTags)
        (Utilities|AddComponenttoMapTagComponents (.Format%20Tag%20 (Utilities|GetandFormatComponentTag _array_element_3 (LocalVariables|GetTagIndex) (LocalVariables|GetActorIndex))) _array_element_3 (LocalVariables|GetMapTagComponents)))))
  (return (LocalVariables|GetMapTagComponents)))

(fn SetPerceptionData
  (params (MapPerceptionData :type Map%20of%20Strings%20to%20Structs))
  (bind _keys (Utilities|Map|Keys MapPerceptionData))
  (for (_array_element _array_index) _keys
    ;[1 1 1] All the components are saved with the a distance higher than the min visible distance. In case they pass the filters, then the true distance is computed
    (LocalVariables|SetCurrentMinDistance (+ (Variables|Default|GetMinVisibleDistance) 1.0))
    (for _array_element_2 (Utilities|Struct|BreakStruct_PerceptionData (.Value (Utilities|Map|Find MapPerceptionData _array_element)))
      (Utilities|FlowControl|Sequence
        (:then_0
          (LocalVariables|SetIsInFOV false))
        (:then_1
          (LocalVariables|SetIsVisible false)
          ;[1 1 1] First Passes the FOV Filter
          (bind _bisinfov (CallFunction|FOVFilter _array_element_2))
          (if _bisinfov
            (LocalVariables|SetIsInFOV true)
            ;[1 1 1] If the component is inside FOV, then the Line of Sight Filter is computed
            (bind _bisvisible (CallFunction|LineOfSightFilter _array_element_2))
            (if _bisvisible
              (LocalVariables|SetIsVisible true)
              ;[1 1 1] If the component is visible, then the distance is computed and saved
              (bind _fdistancetoplayer (CallFunction|GetDistancetoPlayer _array_element_2))
              (if (< _fdistancetoplayer (LocalVariables|GetCurrentMinDistance))
                (LocalVariables|SetCurrentMinDistance _fdistancetoplayer)))))))
    ;[1 1 1] All perception data is stored in a Struct Perception Data, which is mapped inside Map Perception Data using the formatted tag as the key. Separately, component distances are stored in ArrMinDistances to compute the minimum distance in GetChosenComponentsToFlicker
    (Utilities|Struct|SetmembersinStruct_PerceptionData (.Value (Utilities|Map|Find MapPerceptionData _array_element)) (LocalVariables|GetIsInFOV) (LocalVariables|GetIsVisible) (LocalVariables|GetCurrentMinDistance)) ; If at least one of the components is in FOV, FOV is set to True. Same with In Sight
    (Utilities|Array|SetArrayElem (LocalVariables|GetArrMinDistances1) _array_index (LocalVariables|GetCurrentMinDistance) true))
  (return (LocalVariables|GetArrMinDistances1)))

(fn GetChosenComponentstoFlicker
  (params (MapPercpetionData :type Map%20of%20Strings%20to%20Structs) (ArrMinDistances :type Array%20of%20Floats%20%28double-precision%29))
  (bind _returnvalue (Utilities|Array|Length ArrMinDistances))
  (bind (_indexofminvalue _minvalue) (Math|Float|MinOfFloatArray ArrMinDistances))
  (bind _keys (Utilities|Map|Keys MapPercpetionData))
  ;[1 1 1] Choose the smallest betwween the length of the min distances arrayand the total amount of codes sequences
  (if (> _returnvalue (Variables|Default|GetTotalCodeSequences))
    (LocalVariables|SetTotalIndexes (- (Variables|Default|GetTotalCodeSequences) 1))
    (else
      (LocalVariables|SetTotalIndexes (- _returnvalue 1))))
  ;[1 1 1] Loops through each stored perception data entry to find the closest component
  (Utilities|FlowControl|ForLoopwithBreak 0 (LocalVariables|GetTotalIndexes) :!label _label
    (:LoopBody
      (LocalVariables|SetIndexMinValue _indexofminvalue)
      (if (<= _minvalue (Variables|Default|GetMinVisibleDistance))
        ;[1 1 1] Once a component is selected for flickering, its distance is updated to a value higher than MinVisibleDistance to prevent it from being chosen again in the next iteration. The element is not deleted to maintain index consistency
        (Utilities|Array|SetArrayElem ArrMinDistances _indexofminvalue (+ (Variables|Default|GetMinVisibleDistance) 1.0) true) ; Reset that distance to the biggest possible to get, so it wont be chosen again
        ;[1 1 1] Its finally added to the array of chosen components. This array is made of arrays of mesh components
        (Utilities|Array|Add (LocalVariables|GetStructChosenComponents1) (Utilities|Struct|MakeStruct_ArrayMeshComponents (Utilities|Struct|BreakStruct_PerceptionData (.Value (Utilities|Map|Find MapPercpetionData (Utilities|Array|Get(acopy) _keys (LocalVariables|GetIndexMinValue)))))))
        (else
          (goto _label Break))))
    (:Completed
      (return (LocalVariables|GetStructChosenComponents1)))))

(fn ArrangeIntoCodesStruct
  (params (MapPercpetionData :type Map%20of%20Strings%20to%20Structs) (ArrMinDistances :type Array%20of%20Floats%20%28double-precision%29) (ArrStruct_FlickerCodeSequences :type Array%20of%20Struct%20Flicker%20Sequence%20Structures))
  (bind _structchosencomponents (CallFunction|GetChosenComponentstoFlicker MapPercpetionData ArrMinDistances))
  (bind _output_get (LocalVariables|SetStructChosenComponents _structchosencomponents))
  ;[1 1 1] Defines two sets: one with the chosen components arrays (chosenAux) and other with the components already mapped within the flicker sequences, stored in ArrStruct_FlickerCodeSequences
  (for _array_element _output_get
    (Utilities|Set|AddItems (LocalVariables|GetchosenAux) (Utilities|Struct|BreakStruct_ArrayMeshComponents _array_element)))
  (for _array_element_2 ArrStruct_FlickerCodeSequences
    (Utilities|Set|AddItems (LocalVariables|GetcodesAux) (Utilities|Struct|BreakStruct_FlickerSequence _array_element_2)))
  ;[1 1 1] For each sequence in ArrStruct_FlickerCodeSequences, associated mesh components are checked against the chosen components set. If present, they remain linked; otherwise, their overlay material is removed, and new components are assigned
  (for (_array_element_3 _array_index) ArrStruct_FlickerCodeSequences
    (LocalVariables|SetCurrentIndex _array_index)
    (bind _output_get_2 (LocalVariables|SetInChosen (Utilities|Set|Contains (LocalVariables|GetchosenAux) (Utilities|Array|Get(acopy) (.AssociatedMeshComponents (Utilities|Struct|BreakStruct_FlickerSequence _array_element_3))))))
    (if (not _output_get_2)
      (for _array_element_4 (.AssociatedMeshComponents (Utilities|Struct|BreakStruct_FlickerSequence _array_element_3))
        (Rendering|Material|SetOverlayMaterial _array_element_4 0 :!class /Script/Engine.MeshComponent) ; Remove the overlay material with the flickers, on the components that wont flicker now
      )
      (if (Utilities|Array|IsNotEmpty (LocalVariables|GetStructChosenComponents))
        ;[1 1 1] For each chosen component, we check if it is already linked to any flicker sequence. If not, it is a new component that can be assigned to a code sequence.
        (bind (_array_element_5 _array_index_2) (Utilities|Array|ForEachLoopwithBreak (LocalVariables|GetStructChosenComponents) :!label _label)
          (:LoopBody
            (LocalVariables|SetChosenCompIndex _array_index_2)
            (bind _output_get_3 (LocalVariables|SetInCodes (Utilities|Set|Contains (LocalVariables|GetcodesAux) (Utilities|Array|Get(acopy) (Utilities|Struct|BreakStruct_ArrayMeshComponents _array_element_5)))))
            (if (not _output_get_3)
              ;[1 1 1] The mesh components are assigned to that code sequence and removed from the array struct of chosen components and chosenAux
              (bind _structout (Utilities|Struct|SetmembersinStruct_FlickerSequence (Utilities|Array|Get(acopy) ArrStruct_FlickerCodeSequences (LocalVariables|GetCurrentIndex)) (Utilities|Struct|BreakStruct_ArrayMeshComponents (Utilities|Array|Get(acopy) (LocalVariables|GetStructChosenComponents) (LocalVariables|GetChosenCompIndex)))))
              (Utilities|Set|RemoveItems (LocalVariables|GetchosenAux) (Utilities|Struct|BreakStruct_ArrayMeshComponents (Utilities|Array|Get(acopy) (LocalVariables|GetStructChosenComponents) (LocalVariables|GetChosenCompIndex))))
              (Utilities|Array|RemoveIndex (LocalVariables|GetStructChosenComponents) (LocalVariables|GetChosenCompIndex))
              ;[1 1 1] String with codes number that change the mesh components that had associated
              (if (Utilities|Array|IsEmpty (LocalVariables|GetCodesThatChangeComponen))
                (LocalVariables|SetCodesThatChangeComponen (Utilities|String|ToString(Integer) (.SequenceID (Utilities|Struct|BreakStruct_FlickerSequence _structout))))
                (else
                  (LocalVariables|SetCodesThatChangeComponen (Utilities|String|Append (LocalVariables|GetCodesThatChangeComponen) "," (Utilities|String|ToString(Integer) (.SequenceID (Utilities|Struct|BreakStruct_FlickerSequence _structout)))))))
              (for _array_element_6 (.AssociatedMeshComponents (Utilities|Struct|BreakStruct_FlickerSequence _structout))
                (Rendering|Material|SetOverlayMaterial _array_element_6 (.DynamicMaterial (Utilities|Struct|BreakStruct_FlickerSequence _structout)) :!class /Script/Engine.MeshComponent) ; Set the flicker overlay material for tor the components that will flicker
              )
              (goto _label Break)))
          (:Completed
            (if (LocalVariables|GetInCodes)
              ;[1 1 1] Comment
              (Utilities|Struct|SetmembersinStruct_FlickerSequence (Utilities|Array|Get(acopy) ArrStruct_FlickerCodeSequences (LocalVariables|GetCurrentIndex)) (LocalVariables|GetArrEmpty) :!label _label_2))))
        (else
          (goto _label_2)))))
  (return (LocalVariables|GetCodesThatChangeComponen)))