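; Calibration controller that runs the block-based flicker calibration phase once Timeflux delivers code sequences through BP_LSL.
; The received sequences configure BP_FlickerManager, and block duration derives from sequence length, flicker rate, repetitions and pause time.
; A looping timer pauses and resets flickering each block for user recovery, then stops it after the final block.
; Start and end are signaled through BP_LSL's epoch outlet data and event dispatchers.
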(event Custom|CalibrationBegins
  (params (TaskSeqsRec :type String))
  (bind _onetotalblockduration (Variables|Default|GetOneTotalBlockDuration))
  (Default|SetUpFlickers (Variables|Components|GetFlickerManager) (Variables|Default|GetTag) TaskSeqsRec false)
  (Utilities|FlowControl|Delay 1.0)
  (Utilities|DefineBlockValues
    (:%20
      ;[1 1 1] Sends to BP_LSL the commnad to send the event of calibration_ends
      (Utilities|Array|SetArrayElem (Variables|/Game/Flickers_ToImport/Blueprints/BP_LSL.BP_LSL_C|GetOutletData_epochs (Variables|Components|GetBP_LSL)) 0 "calibration_begins")
      (Default|CallCalibrationBegins)
      (Development|PrintString "CALIBRATION BEGINS")
      ;[1 1 1] Calibration is divided in blocks, and are called using a timer
      (Variables|Default|SetCountBlockEvent 0)
      (Utilities|Time|SetTimerbyEvent (EventDispatchers|CreateEvent :!event Custom|Block) _onetotalblockduration true (- 0.0 _onetotalblockduration)))))

(event Custom|Block
  (bind _bp_lsl (Variables|Components|GetBP_LSL))
  (bind _outletdata_epochs (Variables|/Game/Flickers_ToImport/Blueprints/BP_LSL.BP_LSL_C|GetOutletData_epochs _bp_lsl))
  (Development|PrintString "Block")
  ;[1 1 1] Checks if all blocks are done
  (bind _result (Math|Integer|IncrementInt (Variables|Default|GetCountBlockEvent))
    (:%20%20
      (if (> _result (Variables|Default|GetNumberOfBlocks))
        ;[1 1 1] Finalizes the flickering
        (Utilities|FlowControl|Sequence
          (:then_0
            (Default|StopFlickering (Variables|Components|GetFlickerManager) true true)
            ;[1 1 1] Sends to BP_LSL the commnad to send the event of calibration_ends
            (Utilities|FlowControl|Delay 1.0)
            (Utilities|FlowControl|Sequence
              (:then_0
                (Utilities|Array|SetArrayElem _outletdata_epochs 0 "calibration_ends")
                (Development|PrintString "CALIBRATION ENDS"))
              (:then_1
                (Utilities|Array|SetArrayElem _outletdata_epochs 1 "")
                (Default|CallCalibrationEnds))))
          (:then_1
            (Utilities|Time|ClearTimerbyFunctionName 0 "Block") ; The timer that calls the Blocks is stoped
          ))
        (else
          ;[1 1 1] Pausing the flickers to leave the user sme time to recover and blink there eyes if needed
          (Default|PauseFlickering (Variables|Components|GetFlickerManager) (Variables|Default|GetOneBlockPauseDuration) true) ; We reset the index code just in case there is a lag in time or something, and we dont reach to finish our code sequence by the time the timer intializes again the block( )
        )))))

(event EventBeginPlay
  (Utilities|FlowControl|Sequence
    (:then_0
      ;[1 1 1] Retrieves BP_LSL and BP_FlickerManager actors and binds the CalibrationBegins event to handle calibration sequences
      (bind _returnvalue (Actor|GetActorOfClass "/Game/Flickers_ToImport/Blueprints/BP_LSL.BP_LSL_C"))
      (Variables|Components|SetBP_LSL _returnvalue)
      (EventDispatchers|BindEventtoCalibrationSequencesReceived (Variables|Components|GetBP_LSL) (EventDispatchers|CreateEvent :!event Custom|CalibrationBegins)) ; The calibration phase wont start until Timeflux sends the calibration codes
    )
    (:then_1
      (bind _returnvalue_2 (Actor|GetActorOfClass "/Game/Flickers_ToImport/Blueprints/BP_FlickerManager.BP_FlickerManager_C"))
      (Variables|Components|SetFlickerManager _returnvalue_2))))

(fn ConstructionScript)